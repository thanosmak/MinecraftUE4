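; Player controller for a Minecraft-style voxel game that streams terrain chunks around the player and handles block editing and selection.
; Each tick it updates the player's chunk coordinate, then destroys or spawns VoxelActor_BP chunks by CheckRadius, tracked in parallel coordinate and actor arrays.
; Mouse clicks trace from the camera and nudge the hit point to add or remove a voxel in that chunk.
; Number keys and mouse wheel pick the block type, highlighted on the HUD toolbar.
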(event EventBeginPlay
  (CallFunction|Initialize)
  (bind _returnvalue (UserInterface|CreateWidget "/Game/Minecraft/HUD/Master_HUD_BP.Master_HUD_BP_C"))
  (bind _output_get (Variables|Default|SetMaster%20HUD _returnvalue))
  (UserInterface|Viewport|AddtoViewport _output_get 0)
  (Class|Image|SetBrushfromMaterial (Variables|/Game/Minecraft/HUD/Toolbar_Widget_BP.Toolbar_Widget_BP_C|GetB1 (Variables|/Game/Minecraft/HUD/Master_HUD_BP.Master_HUD_BP_C|GetToolbar_Widget_BP_67 _output_get)) "/Game/Minecraft/Materials/Toolbar_Select_M.Toolbar_Select_M"))

(event EventTick
  (params (DeltaSeconds :type Float%20%28single-precision%29))
  (CallFunction|UpdatePosition)
  (CallFunction|RemoveChunk)
  (CallFunction|AddChunck))

(event Input|MouseEvents|MouseWheelUp
  (params (Key :type Key%20Structure :default "None"))
  (bind _master_hud (Variables|Default|GetMaster%20HUD))
  (bind _toolbar_widget_bp_67 (Variables|/Game/Minecraft/HUD/Master_HUD_BP.Master_HUD_BP_C|GetToolbar_Widget_BP_67 _master_hud))
  ;[1 1 1] Input Controls
  (:Pressed
    (Variables|Default|SetblockType (Math|Integer|Clamp(Integer) (+ (Variables|Default|GetblockType) 1) 1 4))
    (Class|Image|SetBrushfromMaterial (Variables|/Game/Minecraft/HUD/Toolbar_Widget_BP.Toolbar_Widget_BP_C|GetB1 (Variables|/Game/Minecraft/HUD/Master_HUD_BP.Master_HUD_BP_C|GetToolbar_Widget_BP_67 (Variables|Default|GetMaster%20HUD))) "/Game/Minecraft/Materials/Toolbar_M.Toolbar_M")
    (Class|Image|SetBrushfromMaterial (Utilities|Select :Index (Variables|Default|GetblockType) :Option%200 0 :Option%201 (Variables|/Game/Minecraft/HUD/Toolbar_Widget_BP.Toolbar_Widget_BP_C|GetB1 _toolbar_widget_bp_67) :Option%202 (Variables|/Game/Minecraft/HUD/Toolbar_Widget_BP.Toolbar_Widget_BP_C|GetB2 _toolbar_widget_bp_67) :Option%203 (Variables|/Game/Minecraft/HUD/Toolbar_Widget_BP.Toolbar_Widget_BP_C|GetB3 _toolbar_widget_bp_67) :Option%204 (Variables|/Game/Minecraft/HUD/Toolbar_Widget_BP.Toolbar_Widget_BP_C|GetB4 _toolbar_widget_bp_67)) "/Game/Minecraft/Materials/Toolbar_Select_M.Toolbar_Select_M")))

(event Input|MouseEvents|MouseWheelDown
  (params (Key :type Key%20Structure :default "None"))
  (bind _master_hud (Variables|Default|GetMaster%20HUD))
  (bind _toolbar_widget_bp_67 (Variables|/Game/Minecraft/HUD/Master_HUD_BP.Master_HUD_BP_C|GetToolbar_Widget_BP_67 _master_hud))
  ;[1 1 1] Input Controls
  (:Pressed
    (Variables|Default|SetblockType (Math|Integer|Clamp(Integer) (+ (Variables|Default|GetblockType) -1) 1 4))
    (Class|Image|SetBrushfromMaterial (Variables|/Game/Minecraft/HUD/Toolbar_Widget_BP.Toolbar_Widget_BP_C|GetB1 (Variables|/Game/Minecraft/HUD/Master_HUD_BP.Master_HUD_BP_C|GetToolbar_Widget_BP_67 (Variables|Default|GetMaster%20HUD))) "/Game/Minecraft/Materials/Toolbar_M.Toolbar_M")
    (Class|Image|SetBrushfromMaterial (Utilities|Select :Index (Variables|Default|GetblockType) :Option%200 0 :Option%201 (Variables|/Game/Minecraft/HUD/Toolbar_Widget_BP.Toolbar_Widget_BP_C|GetB1 _toolbar_widget_bp_67) :Option%202 (Variables|/Game/Minecraft/HUD/Toolbar_Widget_BP.Toolbar_Widget_BP_C|GetB2 _toolbar_widget_bp_67) :Option%203 (Variables|/Game/Minecraft/HUD/Toolbar_Widget_BP.Toolbar_Widget_BP_C|GetB3 _toolbar_widget_bp_67) :Option%204 (Variables|/Game/Minecraft/HUD/Toolbar_Widget_BP.Toolbar_Widget_BP_C|GetB4 _toolbar_widget_bp_67)) "/Game/Minecraft/Materials/Toolbar_Select_M.Toolbar_Select_M")))

(event Input|KeyboardEvents|1
  (params (Key :type Key%20Structure :default "None"))
  (bind _master_hud (Variables|Default|GetMaster%20HUD))
  (bind _toolbar_widget_bp_67 (Variables|/Game/Minecraft/HUD/Master_HUD_BP.Master_HUD_BP_C|GetToolbar_Widget_BP_67 _master_hud))
  ;[1 1 1] Input Controls
  (:Pressed
    (Variables|Default|SetblockType 1)
    (Class|Image|SetBrushfromMaterial (Variables|/Game/Minecraft/HUD/Toolbar_Widget_BP.Toolbar_Widget_BP_C|GetB1 (Variables|/Game/Minecraft/HUD/Master_HUD_BP.Master_HUD_BP_C|GetToolbar_Widget_BP_67 (Variables|Default|GetMaster%20HUD))) "/Game/Minecraft/Materials/Toolbar_M.Toolbar_M")
    (Class|Image|SetBrushfromMaterial (Utilities|Select :Index (Variables|Default|GetblockType) :Option%200 0 :Option%201 (Variables|/Game/Minecraft/HUD/Toolbar_Widget_BP.Toolbar_Widget_BP_C|GetB1 _toolbar_widget_bp_67) :Option%202 (Variables|/Game/Minecraft/HUD/Toolbar_Widget_BP.Toolbar_Widget_BP_C|GetB2 _toolbar_widget_bp_67) :Option%203 (Variables|/Game/Minecraft/HUD/Toolbar_Widget_BP.Toolbar_Widget_BP_C|GetB3 _toolbar_widget_bp_67) :Option%204 (Variables|/Game/Minecraft/HUD/Toolbar_Widget_BP.Toolbar_Widget_BP_C|GetB4 _toolbar_widget_bp_67)) "/Game/Minecraft/Materials/Toolbar_Select_M.Toolbar_Select_M")))

(event Input|KeyboardEvents|2
  (params (Key :type Key%20Structure :default "None"))
  (bind _master_hud (Variables|Default|GetMaster%20HUD))
  (bind _toolbar_widget_bp_67 (Variables|/Game/Minecraft/HUD/Master_HUD_BP.Master_HUD_BP_C|GetToolbar_Widget_BP_67 _master_hud))
  ;[1 1 1] Input Controls
  (:Pressed
    (Variables|Default|SetblockType 2)
    (Class|Image|SetBrushfromMaterial (Variables|/Game/Minecraft/HUD/Toolbar_Widget_BP.Toolbar_Widget_BP_C|GetB1 (Variables|/Game/Minecraft/HUD/Master_HUD_BP.Master_HUD_BP_C|GetToolbar_Widget_BP_67 (Variables|Default|GetMaster%20HUD))) "/Game/Minecraft/Materials/Toolbar_M.Toolbar_M")
    (Class|Image|SetBrushfromMaterial (Utilities|Select :Index (Variables|Default|GetblockType) :Option%200 0 :Option%201 (Variables|/Game/Minecraft/HUD/Toolbar_Widget_BP.Toolbar_Widget_BP_C|GetB1 _toolbar_widget_bp_67) :Option%202 (Variables|/Game/Minecraft/HUD/Toolbar_Widget_BP.Toolbar_Widget_BP_C|GetB2 _toolbar_widget_bp_67) :Option%203 (Variables|/Game/Minecraft/HUD/Toolbar_Widget_BP.Toolbar_Widget_BP_C|GetB3 _toolbar_widget_bp_67) :Option%204 (Variables|/Game/Minecraft/HUD/Toolbar_Widget_BP.Toolbar_Widget_BP_C|GetB4 _toolbar_widget_bp_67)) "/Game/Minecraft/Materials/Toolbar_Select_M.Toolbar_Select_M")))

(event Input|KeyboardEvents|3
  (params (Key :type Key%20Structure :default "None"))
  (bind _master_hud (Variables|Default|GetMaster%20HUD))
  (bind _toolbar_widget_bp_67 (Variables|/Game/Minecraft/HUD/Master_HUD_BP.Master_HUD_BP_C|GetToolbar_Widget_BP_67 _master_hud))
  ;[1 1 1] Input Controls
  (:Pressed
    (Variables|Default|SetblockType 3)
    (Class|Image|SetBrushfromMaterial (Variables|/Game/Minecraft/HUD/Toolbar_Widget_BP.Toolbar_Widget_BP_C|GetB1 (Variables|/Game/Minecraft/HUD/Master_HUD_BP.Master_HUD_BP_C|GetToolbar_Widget_BP_67 (Variables|Default|GetMaster%20HUD))) "/Game/Minecraft/Materials/Toolbar_M.Toolbar_M")
    (Class|Image|SetBrushfromMaterial (Utilities|Select :Index (Variables|Default|GetblockType) :Option%200 0 :Option%201 (Variables|/Game/Minecraft/HUD/Toolbar_Widget_BP.Toolbar_Widget_BP_C|GetB1 _toolbar_widget_bp_67) :Option%202 (Variables|/Game/Minecraft/HUD/Toolbar_Widget_BP.Toolbar_Widget_BP_C|GetB2 _toolbar_widget_bp_67) :Option%203 (Variables|/Game/Minecraft/HUD/Toolbar_Widget_BP.Toolbar_Widget_BP_C|GetB3 _toolbar_widget_bp_67) :Option%204 (Variables|/Game/Minecraft/HUD/Toolbar_Widget_BP.Toolbar_Widget_BP_C|GetB4 _toolbar_widget_bp_67)) "/Game/Minecraft/Materials/Toolbar_Select_M.Toolbar_Select_M")))

(event Input|KeyboardEvents|4
  (params (Key :type Key%20Structure :default "None"))
  (bind _master_hud (Variables|Default|GetMaster%20HUD))
  (bind _toolbar_widget_bp_67 (Variables|/Game/Minecraft/HUD/Master_HUD_BP.Master_HUD_BP_C|GetToolbar_Widget_BP_67 _master_hud))
  ;[1 1 1] Input Controls
  (:Pressed
    (Variables|Default|SetblockType 4)
    (Class|Image|SetBrushfromMaterial (Variables|/Game/Minecraft/HUD/Toolbar_Widget_BP.Toolbar_Widget_BP_C|GetB1 (Variables|/Game/Minecraft/HUD/Master_HUD_BP.Master_HUD_BP_C|GetToolbar_Widget_BP_67 (Variables|Default|GetMaster%20HUD))) "/Game/Minecraft/Materials/Toolbar_M.Toolbar_M")
    (Class|Image|SetBrushfromMaterial (Utilities|Select :Index (Variables|Default|GetblockType) :Option%200 0 :Option%201 (Variables|/Game/Minecraft/HUD/Toolbar_Widget_BP.Toolbar_Widget_BP_C|GetB1 _toolbar_widget_bp_67) :Option%202 (Variables|/Game/Minecraft/HUD/Toolbar_Widget_BP.Toolbar_Widget_BP_C|GetB2 _toolbar_widget_bp_67) :Option%203 (Variables|/Game/Minecraft/HUD/Toolbar_Widget_BP.Toolbar_Widget_BP_C|GetB3 _toolbar_widget_bp_67) :Option%204 (Variables|/Game/Minecraft/HUD/Toolbar_Widget_BP.Toolbar_Widget_BP_C|GetB4 _toolbar_widget_bp_67)) "/Game/Minecraft/Materials/Toolbar_Select_M.Toolbar_Select_M")))

(event Input|MouseEvents|LeftMouseButton
  (params (Key :type Key%20Structure :default "None"))
  (bind _returnvalue (Game|GetPlayerCameraManager 0))
  (bind _returnvalue_2 (Camera|GetCameraLocation _returnvalue))
  (:Released
    (Variables|Default|SetisAdding false)
    (bind _outhit (Collision|LineTraceByChannel _returnvalue_2 (+ _returnvalue_2 (* (Transformation|GetActorForwardVector _returnvalue) 6e+02)) "TraceTypeQuery1" false 0 "None"))
    (Class|VoxelActor|SetVoxel (Utilities|Array|Get(acopy) (Variables|Default|Getchunks) (Utilities|Array|FindItem (Variables|Default|GetchunkChords) (Math|Vector2D|MakeVector2D (Math|Conversions|ToFloat(Integer) (Math|Float|Floor (.x (/ (+ (+ (.Location (Collision|BreakHitResult _outhit)) (* (Math|Vector|GetUnitDirection(Vector) (.Location (Collision|BreakHitResult _outhit)) _returnvalue_2) (- (* (Math|Conversions|ToFloat(Boolean) (Variables|Default|GetisAdding)) 2.0) 1.0))) "50.000000,50.000000,50.000000") (Variables|Default|GetchunkSize))))) (Math|Conversions|ToFloat(Integer) (Math|Float|Floor (.y (/ (+ (+ (.Location (Collision|BreakHitResult _outhit)) (* (Math|Vector|GetUnitDirection(Vector) (.Location (Collision|BreakHitResult _outhit)) _returnvalue_2) (- (* (Math|Conversions|ToFloat(Boolean) (Variables|Default|GetisAdding)) 2.0) 1.0))) "50.000000,50.000000,50.000000") (Variables|Default|GetchunkSize)))))))) (+ (* (Transformation|GetActorLocation (Utilities|Array|Get(acopy) (Variables|Default|Getchunks) (Utilities|Array|FindItem (Variables|Default|GetchunkChords) (Math|Vector2D|MakeVector2D (Math|Conversions|ToFloat(Integer) (Math|Float|Floor (.x (/ (+ (+ (.Location (Collision|BreakHitResult _outhit)) (* (Math|Vector|GetUnitDirection(Vector) (.Location (Collision|BreakHitResult _outhit)) _returnvalue_2) (- (* (Math|Conversions|ToFloat(Boolean) (Variables|Default|GetisAdding)) 2.0) 1.0))) "50.000000,50.000000,50.000000") (Variables|Default|GetchunkSize))))) (Math|Conversions|ToFloat(Integer) (Math|Float|Floor (.y (/ (+ (+ (.Location (Collision|BreakHitResult _outhit)) (* (Math|Vector|GetUnitDirection(Vector) (.Location (Collision|BreakHitResult _outhit)) _returnvalue_2) (- (* (Math|Conversions|ToFloat(Boolean) (Variables|Default|GetisAdding)) 2.0) 1.0))) "50.000000,50.000000,50.000000") (Variables|Default|GetchunkSize))))))))) -1.0) (+ (.Location (Collision|BreakHitResult _outhit)) (* (Math|Vector|GetUnitDirection(Vector) (.Location (Collision|BreakHitResult _outhit)) _returnvalue_2) (- (* (Math|Conversions|ToFloat(Boolean) (Variables|Default|GetisAdding)) 2.0) 1.0))) (* "0.500000,0.500000,0.500000" (Math|Conversions|ToFloat(Integer) (Variables|Settings|GetvoxelSize)))) (select (Variables|Default|GetisAdding) (Variables|Default|GetblockType) (Variables|Default|GetremoveBlockValue)))))

(event Input|MouseEvents|RightMouseButton
  (params (Key :type Key%20Structure :default "None"))
  (bind _returnvalue (Game|GetPlayerCameraManager 0))
  (bind _returnvalue_2 (Camera|GetCameraLocation _returnvalue))
  (:Released
    (Variables|Default|SetisAdding true)
    (bind _outhit (Collision|LineTraceByChannel _returnvalue_2 (+ _returnvalue_2 (* (Transformation|GetActorForwardVector _returnvalue) 6e+02)) "TraceTypeQuery1" false 0 "None"))
    (Class|VoxelActor|SetVoxel (Utilities|Array|Get(acopy) (Variables|Default|Getchunks) (Utilities|Array|FindItem (Variables|Default|GetchunkChords) (Math|Vector2D|MakeVector2D (Math|Conversions|ToFloat(Integer) (Math|Float|Floor (.x (/ (+ (+ (.Location (Collision|BreakHitResult _outhit)) (* (Math|Vector|GetUnitDirection(Vector) (.Location (Collision|BreakHitResult _outhit)) _returnvalue_2) (- (* (Math|Conversions|ToFloat(Boolean) (Variables|Default|GetisAdding)) 2.0) 1.0))) "50.000000,50.000000,50.000000") (Variables|Default|GetchunkSize))))) (Math|Conversions|ToFloat(Integer) (Math|Float|Floor (.y (/ (+ (+ (.Location (Collision|BreakHitResult _outhit)) (* (Math|Vector|GetUnitDirection(Vector) (.Location (Collision|BreakHitResult _outhit)) _returnvalue_2) (- (* (Math|Conversions|ToFloat(Boolean) (Variables|Default|GetisAdding)) 2.0) 1.0))) "50.000000,50.000000,50.000000") (Variables|Default|GetchunkSize)))))))) (+ (* (Transformation|GetActorLocation (Utilities|Array|Get(acopy) (Variables|Default|Getchunks) (Utilities|Array|FindItem (Variables|Default|GetchunkChords) (Math|Vector2D|MakeVector2D (Math|Conversions|ToFloat(Integer) (Math|Float|Floor (.x (/ (+ (+ (.Location (Collision|BreakHitResult _outhit)) (* (Math|Vector|GetUnitDirection(Vector) (.Location (Collision|BreakHitResult _outhit)) _returnvalue_2) (- (* (Math|Conversions|ToFloat(Boolean) (Variables|Default|GetisAdding)) 2.0) 1.0))) "50.000000,50.000000,50.000000") (Variables|Default|GetchunkSize))))) (Math|Conversions|ToFloat(Integer) (Math|Float|Floor (.y (/ (+ (+ (.Location (Collision|BreakHitResult _outhit)) (* (Math|Vector|GetUnitDirection(Vector) (.Location (Collision|BreakHitResult _outhit)) _returnvalue_2) (- (* (Math|Conversions|ToFloat(Boolean) (Variables|Default|GetisAdding)) 2.0) 1.0))) "50.000000,50.000000,50.000000") (Variables|Default|GetchunkSize))))))))) -1.0) (+ (.Location (Collision|BreakHitResult _outhit)) (* (Math|Vector|GetUnitDirection(Vector) (.Location (Collision|BreakHitResult _outhit)) _returnvalue_2) (- (* (Math|Conversions|ToFloat(Boolean) (Variables|Default|GetisAdding)) 2.0) 1.0))) (* "0.500000,0.500000,0.500000" (Math|Conversions|ToFloat(Integer) (Variables|Settings|GetvoxelSize)))) (select (Variables|Default|GetisAdding) (Variables|Default|GetblockType) (Variables|Default|GetremoveBlockValue)))))

(fn ConstructionScript)

(fn UpdatePosition
  (bind _chunksize (Variables|Default|GetchunkSize))
  (bind _returnvalue (Math|Conversions|ToFloat(Integer) _chunksize))
  (bind _output_get (Variables|Default|SetcharacterPosition (* (Transformation|GetActorLocation (Game|Player|GetPlayerPawn 0)) "1.000000,1.000000,0.000000")))
  (if (or (!= (Variables|Default|GetchunkX) (Math|Float|Floor (/ (.X (Math|Vector|BreakVector _output_get)) _returnvalue))) (!= (Variables|Default|GetchunkY) (Math|Float|Floor (/ (.Y (Math|Vector|BreakVector _output_get)) _returnvalue))))
    (Variables|Default|SetchunkX (Math|Float|Floor (/ (.X (Math|Vector|BreakVector _output_get)) _returnvalue)))
    (Variables|Default|SetchunkY (Math|Float|Floor (/ (.Y (Math|Vector|BreakVector _output_get)) _returnvalue)))
    (return true)
    (else
      (return false))))

(fn Initialize
  (bind _output_get (Variables|Default|SetchunkSize (* (Variables|Settings|GetchunkLineElements) (Variables|Settings|GetvoxelSize))))
  (Variables|Default|SetchunkSizeHalf (/ _output_get 1)))

(fn AddChunck
  (bind _chunksize (Variables|Default|GetchunkSize))
  (bind _renderrange (Variables|Settings|GetrenderRange))
  (bind _chunksizehalf (Variables|Default|GetchunkSizeHalf))
  (bind _chunkchords (Variables|Default|GetchunkChords))
  (bind _returnvalue (Math|Conversions|ToFloat(Integer) _chunksize))
  (bind _returnvalue_2 (Math|Conversions|ToFloat(Integer) _chunksizehalf))
  (bind _returnvalue_3 (* _renderrange -1))
  (for _index (range _returnvalue_3 _renderrange) ; X
    (for _index_2 (range _returnvalue_3 _renderrange) ; Y
      (if (Utilities|CheckRadius (+ (* (+ _index (Variables|Default|GetchunkX)) _returnvalue) _returnvalue_2) (+ (* (+ _index_2 (Variables|Default|GetchunkY)) _returnvalue) _returnvalue_2))
        (if (not (Utilities|Array|ContainsItem _chunkchords (Math|Vector2D|MakeVector2D (Math|Conversions|ToFloat(Integer) (+ _index (Variables|Default|GetchunkX))) (Math|Conversions|ToFloat(Integer) (+ _index_2 (Variables|Default|GetchunkY))))))
          (Utilities|Array|Add _chunkchords (Math|Vector2D|MakeVector2D (Math|Conversions|ToFloat(Integer) (+ _index (Variables|Default|GetchunkX))) (Math|Conversions|ToFloat(Integer) (+ _index_2 (Variables|Default|GetchunkY)))))
          (bind _returnvalue_4 (Game|SpawnActorfromClass "/Game/Minecraft/VoxelActor_BP.VoxelActor_BP_C" (Math|Conversions|ToTransform(Vector) (Math|Vector|MakeVector (* (+ _index (Variables|Default|GetchunkX)) _returnvalue) (* (+ _index_2 (Variables|Default|GetchunkY)) _returnvalue) 0.0)) "Undefined" 0 (Variables|Settings|GetrandomSeed) (Variables|Settings|GetvoxelSize) (Variables|Settings|GetchunkLineElements) (+ _index (Variables|Default|GetchunkX)) (+ _index_2 (Variables|Default|GetchunkY)) 4.0 0))
          (Utilities|Array|Add (Variables|Default|Getchunks) _returnvalue_4))))))

(fn RemoveChunk
  (bind _chunksize (Variables|Default|GetchunkSize))
  (bind _chunksizehalf (Variables|Default|GetchunkSizeHalf))
  (bind _chunks (Variables|Default|Getchunks))
  (bind _returnvalue (Math|Conversions|ToFloat(Integer) _chunksizehalf))
  (for (_array_element _array_index) (Variables|Default|GetchunkChords)
    (if (not (Utilities|CheckRadius (+ (* _chunksize (.X (Math|Vector2D|BreakVector2D _array_element))) _returnvalue) (+ (* _chunksize (.Y (Math|Vector2D|BreakVector2D _array_element))) _returnvalue)))
      (Actor|DestroyActor (Utilities|Array|Get(acopy) _chunks _array_index))
      (Utilities|Array|RemoveIndex (Variables|Default|GetchunkChords) _array_index)
      (Utilities|Array|RemoveIndex _chunks _array_index))))